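; Actor Blueprint that manages a pool of enemy cars and places them on road segments.
; SpawnCar moves the next car in the Cars array to a random start position, transformed into the given segment's space, and matches the segment's rotation.
; The index then advances through IncrementArrayIndex, so existing cars are reused rather than new ones spawned.
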(event Custom|SpawnCar
  (params (RoadSegment :type Road%20Segment%20Object%20Reference))
  (bind _cars (Variables|Default|GetCars))
  (Transformation|SetActorLocationAndRotation (Utilities|Array|Get(acopy) _cars (Variables|Default|GetCarIndex)) (Math|Transform|TransformLocation (Transformation|GetActorTransform RoadSegment) (.OutItem (Utilities|Array|Random (Variables|Default|GetStartPositions)))) (Transformation|GetActorRotation RoadSegment))
  (bind _output (CallFunction|IncrementArrayIndex _cars (Variables|Default|GetCarIndex)))
  (Variables|Default|SetCarIndex _output))

(fn ConstructionScript)