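; CameraRig is the StreetRacer player rig, moving forward while driving and carrying the car as a laterally shiftable component.
; It registers with the controller and game mode and exposes begin, end and reset events.
; A buffered turn matching an overlapped tagged trigger starts a timeline-driven 90-degree rotation, snaps the rig onto the segment, redirects movement and requests new road from RoadManager.
; Overlapping a Kill-tagged component ends the game.
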(event OnComponentBeginOverlap(Box)
  (params (OverlappedComponent :type Primitive%20Component%20Object%20Reference) (OtherActor :type Actor%20Object%20Reference) (OtherComp :type Primitive%20Component%20Object%20Reference) (OtherBodyIndex :type Integer) (bFromSweep :type Boolean) (SweepResult :type Hit%20Result%20Structure%20%28by%20ref%29))
  (CallFunction|TurnCollision OtherActor OtherComp)
  (CallFunction|KillCollision OtherComp))

(event Custom|BeginGame
  (Development|PrintString "Begin Driving")
  (Variables|Default|SetDriving true))

(event Custom|EndGame
  (Development|PrintString "Stop Driving")
  (Variables|Default|SetDriving false))

(event Custom|ResetGame
  (Transformation|SetActorLocation "0, 0, 0" false false)
  (Transformation|SetActorRotation "0, 0, 0")
  (Variables|Default|SetCameraMoveDirection (Math|Vector|GetForwardVector (Transformation|GetActorRotation)))
  (Transformation|SetRelativeLocation (Variables|Default|GetPlayerCar) "0, 0, 0" false false)
  (Variables|Default|SetCurrentCarOffset 0.0))

(event Custom|Turn
  (params (LeftTurn :type Boolean))
  (if LeftTurn
    (Variables|Default|SetLeftTurn true)
    (Variables|Default|SetRightTurn false)
    (else
      (Variables|Default|SetRightTurn true)
      (Variables|Default|SetLeftTurn false))))

(event Custom|Rotate
  (params (Rotation :type Rotator))
  (bind _returnvalue (Transformation|GetActorRotation))
  (bind _output_get (Variables|Default|SetCameraTargetRotation (Math|Rotator|CombineRotators _returnvalue Rotation)))
  (bind _alpha (Timeline|RotateCamera PlayFromStart)
    (:Update
      (Transformation|SetActorRotation (Math|Rotator|Lerp(Rotator) _returnvalue _output_get _alpha true)))))

(event Custom|Shift
  (params (Delta :type Float%20%28double-precision%29))
  (if (Variables|Default|GetDriving)
    (bind _output_get (Variables|Default|SetCurrentCarOffset (+ (* Delta 1.0) (Variables|Default|GetCurrentCarOffset))))
    (Transformation|SetRelativeLocation (Variables|Default|GetPlayerCar) (Math|Vector|MakeVector 0.0 _output_get 0.0) false false)))

(event Custom|TurnCollision
  (params (OtherActor :type Actor%20Object%20Reference) (OtherComponent :type Actor%20Component%20Object%20Reference))
  (if (and (Components|ComponentHasTag OtherComponent "LeftTurn") (Variables|Default|GetLeftTurn))
    (CallFunction|Rotate "0.000000,-90.000000,0.000000")
    (Transformation|SetActorLocation (Math|Transform|TransformLocation (Transformation|GetActorTransform OtherActor) (Math|Vector|MakeVector (/ (Variables|/Game/Blueprints/RoadManager/RoadManager.RoadManager_C|GetRoadSegmentLength (Variables|Default|GetRoadManager)) 2.0) 0.0 0.0)) false false :!label _label)
    (Variables|Default|SetCameraMoveDirection (Math|Vector|GetForwardVector (Variables|Default|GetCameraTargetRotation)))
    (Default|SpawnRoad (Variables|Default|GetRoadManager))
    (Variables|Default|SetLeftTurn false)
    (Variables|Default|SetRightTurn false)
    (elif (and (Components|ComponentHasTag OtherComponent "RightTurn") (Variables|Default|GetRightTurn))
      (CallFunction|Rotate "0.000000,90.000000,0.000000")
      (goto _label))))

(event Custom|KillCollision
  (params (OtherComponent :type Actor%20Component%20Object%20Reference))
  (if (Components|ComponentHasTag OtherComponent "Kill")
    (Default|EndGame (Variables|Default|GetStreetRacerGameMode))))

(event EventBeginPlay
  (bind _self self)
  (bind _asstreet_racer_controller (Utilities|Casting|CastToStreetRacerController (Game|GetPlayerController 0)))
  (Default|SetCar _asstreet_racer_controller _self)
  (bind _asstreet_racer_game_mode (Utilities|Casting|CastToStreetRacerGameMode (Game|GetGameMode)))
  (bind _output_get (Variables|Default|SetStreetRacerGameMode _asstreet_racer_game_mode))
  (Default|SetPlayerCar _asstreet_racer_game_mode _self))

(event EventTick
  (params (DeltaSeconds :type Float%20%28single-precision%29))
  (if (Variables|Default|GetDriving)
    (Transformation|SetActorLocation (+ (Transformation|GetActorLocation) (* (* DeltaSeconds (Variables|Default|GetSpeed)) (Variables|Default|GetCameraMoveDirection))) false false)))

(fn ConstructionScript)