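; Player controller for a street racer game that lets the player start and end a game through input actions.
; On BeginPlay it adds the StreetRacerMappingContext to Enhanced Input and caches the StreetRacerGameMode.
; The StartGame and EndGame actions print a debug string and call the matching functions on that game mode.
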(event Input|EnhancedActionEvents|EnhancedInputActionStartGame
  (params (ActionValue :type Boolean) (ElapsedSeconds :type Float%20%28double-precision%29) (TriggeredSeconds :type Float%20%28double-precision%29) (InputAction :type Input%20Action%20Object%20Reference :default "/Game/Blueprints/StartGame.StartGame"))
  (:Triggered
    (Development|PrintString "Start Game")
    (Default|StartGame (Variables|Default|GetStreetRacerGameMode))))

(event Input|EnhancedActionEvents|EnhancedInputActionEndGame
  (params (ActionValue :type Boolean) (ElapsedSeconds :type Float%20%28double-precision%29) (TriggeredSeconds :type Float%20%28double-precision%29) (InputAction :type Input%20Action%20Object%20Reference :default "/Game/Blueprints/EndGame.EndGame"))
  (:Triggered
    (Development|PrintString "End Game")
    (Default|EndGame (Variables|Default|GetStreetRacerGameMode))))

(event EventBeginPlay
  (Input|AddMappingContext (PlayerController|LocalPlayerSubsystems|GetEnhancedInputLocalPlayerSubsystem) "/Game/Blueprints/StreetRacerMappingContext.StreetRacerMappingContext" 0 "(bIgnoreAllPressedKeysUntilRelease=True,bForceImmediately=False)")
  (bind _asstreet_racer_game_mode (Utilities|Casting|CastToStreetRacerGameMode (Game|GetGameMode)))
  (Variables|Default|SetStreetRacerGameMode _asstreet_racer_game_mode))

(event EventTick
  (params (DeltaSeconds :type Float%20%28single-precision%29)))

(fn ConstructionScript)