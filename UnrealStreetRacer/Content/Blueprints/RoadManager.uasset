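; RoadManager keeps a road running under a travelling car by recycling a fixed pool of road segment actors.
; Its CarTravel event counts travelled distance down from the segment length.
; When the countdown runs out, it resets, advances the total distance by one segment and moves the next segment in the wrapping array to that point on the Y axis.
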(event Custom|CarTravel
  (params (Distance :type Float%20%28double-precision%29))
  (bind _roadsegments (Variables|Default|GetRoadSegments))
  (bind _roadsegmentlength (Variables|Default|GetRoadSegmentLength))
  (bind _output_get (Variables|Default|SetDistanceTillNextSpawn (- (Variables|Default|GetDistanceTillNextSpawn) Distance)))
  (if (<= _output_get 0.0)
    (Variables|Default|SetDistanceTillNextSpawn _roadsegmentlength)
    (Variables|Default|SetTotalDistanceTraveled (+ (Variables|Default|GetTotalDistanceTraveled) _roadsegmentlength))
    (bind _output_get_2 (Variables|Default|SetRoadSegmentIndex (+ (Variables|Default|GetRoadSegmentIndex) 1)))
    (if (>= _output_get_2 (Utilities|Array|Length _roadsegments))
      (Variables|Default|SetRoadSegmentIndex 0))
    (Transformation|SetActorLocation (Utilities|Array|Get(acopy) _roadsegments _output_get_2) (Math|Vector|MakeVector 0.0 (Variables|Default|GetTotalDistanceTraveled) 0.0) false false)))

(fn ConstructionScript)