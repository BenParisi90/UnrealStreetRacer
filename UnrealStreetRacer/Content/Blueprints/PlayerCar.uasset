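; Player car for an endless street racer that drives forward automatically along spawned road segments.
; Steering offsets and yaws the car model sideways, while the e-brake exaggerates yaw and plays a drift loop.
; Steering with the e-brake in tagged turn volumes snaps the car to the corner, lerps the camera rig 90 degrees and spawns road.
; A missed turn leaves the camera behind; hitting Kill components ends the game with an explosion.
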(event OnComponentBeginOverlap(Box)
  (params (OverlappedComponent :type Primitive%20Component%20Object%20Reference) (OtherActor :type Actor%20Object%20Reference) (OtherComp :type Primitive%20Component%20Object%20Reference) (OtherBodyIndex :type Integer) (bFromSweep :type Boolean) (SweepResult :type Hit%20Result%20Structure%20%28by%20ref%29))
  (CallFunction|TurnCollision OtherActor OtherComp)
  (CallFunction|KillCollision OtherComp))

(event Custom|BeginGame
  (Development|PrintString "Begin Driving")
  (Variables|Default|SetDriving true)
  (bind _returnvalue (Audio|SpawnSound2D "/Game/Audio/EngineLoop.EngineLoop" 1.0 1.0 0.0 0)))

(event Custom|EndGame
  (Development|PrintString "Stop Driving")
  (Variables|Default|SetDriving false)
  (Components|Activation|SetActive (stale Custom|BeginGame _returnvalue) false false))

(event Custom|StartDriftingIfNeeded
  (if (not (Variables|Default|GetDrifting))
    (Variables|Default|SetDrifting true)
    (bind _returnvalue (Audio|SpawnSound2D "/Game/Audio/SkidLoop.SkidLoop" 1.0 1.0 0.0 0))
    (Variables|Default|SetDriftSound _returnvalue)))

(event Custom|EBreak
  (params (Engage :type Boolean))
  (Variables|Default|SetEBreakEngaged Engage))

(event Custom|StopDriftingIfPossible
  (if (Variables|Default|GetDrifting)
    (Variables|Default|SetDrifting false)
    (Audio|Components|Audio|Stop (Variables|Default|GetDriftSound))))

(event Custom|ResetGame
  (bind _camerarig (Variables|Default|GetCameraRig))
  (Transformation|SetActorLocation "0, 0, 0" false false)
  (Transformation|SetActorRotation "0, 0, 0")
  (Transformation|SetRelativeLocationAndRotation (Variables|Default|GetPlayerCarModel) "0, 0, 0" "0, 0, 0" false false)
  (Variables|Default|SetCurrentCarOffset 0.0)
  (Variables|Default|SetMoveDirection (Transformation|GetActorForwardVector))
  (Variables|Default|SetCameraTargetRotation "0, 0, 0")
  (Transformation|AttachActorToActor _camerarig self "None" "KeepRelative" "KeepRelative" "KeepRelative" true)
  (Transformation|SetActorRelativeLocation _camerarig)
  (Transformation|SetActorRelativeRotation _camerarig)
  (Rendering|SetVisibility (Variables|Default|GetHeadlight) true false))

(event Custom|Turn
  (params (LeftTurn :type Boolean) (EngageTurn :type Boolean))
  (if LeftTurn
    (Variables|Default|SetLeftTurn EngageTurn)
    (else
      (Variables|Default|SetRightTurn EngageTurn))))

(event Custom|Rotate
  (params (Rotation :type Rotator))
  (bind _camerarig (Variables|Default|GetCameraRig))
  (bind _returnvalue (Transformation|GetActorRotation _camerarig))
  (bind _output_get (Variables|Default|SetCameraTargetRotation (Math|Rotator|CombineRotators _returnvalue Rotation)))
  (bind _alpha (Timeline|RotateCamera PlayFromStart)
    (:Update
      (Transformation|SetActorRotation (Variables|Default|GetCameraRig) (Math|Rotator|Lerp(Rotator) _returnvalue _output_get _alpha true)))))

(event Custom|TurnPlayerCar
  (params (DeltaSeconds :type Float%20%28double-precision%29))
  (if (Variables|Default|GetDriving)
    (if (not (Variables|Default|GetEBreakEngaged))
      (CallFunction|StopDriftingifPossible))
    (Variables|Default|SetCarModelRotation 0.0)
    (Variables|Default|SetCarOffsetMultiplier 0.0)
    (if (Variables|Default|GetLeftTurn)
      (Variables|Default|SetCarModelRotation -15.0)
      (Variables|Default|SetCarOffsetMultiplier -1.0)
      (elif (Variables|Default|GetRightTurn)
        (Variables|Default|SetCarModelRotation 15.0)
        (Variables|Default|SetCarOffsetMultiplier 1.0)
        (else
          (CallFunction|StopDriftingifPossible))))
    (if (Variables|Default|GetEBreakEngaged)
      (bind _output_get (Variables|Default|SetCarModelRotation (* (stale _output_get) 4.0)))
      (bind _output_get_2 (Variables|Default|SetCarOffsetMultiplier (* (stale _output_get_2) 0.25)))
      (CallFunction|StartDriftingifNeeded))
    (Transformation|SetRelativeRotation (Variables|Default|GetPlayerCarModel) (Math|Rotator|CombineRotators (Variables|Default|GetCameraTargetRotation) (Math|Rotator|MakeRotator 0.0 0.0 (Variables|Default|GetCarModelRotation))) false false)
    (bind _output_get_3 (Variables|Default|SetCurrentCarOffset (+ (stale _output_get_3) (* (Variables|Default|GetTurnSpeed) (Variables|Default|GetCarOffsetMultiplier) DeltaSeconds))))
    (Transformation|SetRelativeLocation (Variables|Default|GetPlayerCarModel) (* (Variables|Default|GetCurrentCarOffset) (Math|Vector|GetRightVector (Variables|Default|GetCameraTargetRotation))) false false)))

(event Custom|TurnCollision
  (params (OtherActor :type Actor%20Object%20Reference) (OtherComponent :type Actor%20Component%20Object%20Reference))
  (bind _returnvalue (Components|ComponentHasTag OtherComponent "RightTurn"))
  (bind _returnvalue_2 (Components|ComponentHasTag OtherComponent "LeftTurn"))
  (bind _ebreakengaged (Variables|Default|GetEBreakEngaged))
  (if (Math|Boolean|ANDBoolean (Variables|Default|GetCanTurnCorner) (Variables|Default|GetDriving) (or _returnvalue_2 _returnvalue))
    (if (Math|Boolean|ANDBoolean _returnvalue_2 (Variables|Default|GetLeftTurn) _ebreakengaged)
      (CallFunction|Rotate "0.000000,-90.000000,0.000000")
      (Transformation|SetRelativeRotation (Variables|Default|GetPlayerCarModel) (Variables|Default|GetCameraTargetRotation) false false :!label _label)
      (Variables|Default|SetMoveDirection (Math|Vector|GetForwardVector (Variables|Default|GetCameraTargetRotation)))
      (Transformation|SetActorLocation (Math|Transform|TransformLocation (Transformation|GetActorTransform OtherActor) (Math|Vector|MakeVector (/ (Variables|/Game/Blueprints/RoadManager/RoadManager.RoadManager_C|GetRoadSegmentLength (Variables|Default|GetRoadManager)) 2.0) 0.0 0.0)) false false)
      (Default|SpawnRoad (Variables|Default|GetRoadManager))
      (CallFunction|PreventTurning 1.0)
      (elif (Math|Boolean|ANDBoolean _returnvalue (Variables|Default|GetRightTurn) _ebreakengaged)
        (CallFunction|Rotate "0.000000,90.000000,0.000000")
        (goto _label)
        (else
          (Transformation|AttachActorToActor (Variables|Default|GetCameraRig) (Variables|Default|GetRoadManager) "None" "KeepWorld" "KeepWorld" "KeepWorld" false))))))

(event Custom|KillCollision
  (params (OtherComponent :type Actor%20Component%20Object%20Reference))
  (if (and (Components|ComponentHasTag OtherComponent "Kill") (Variables|Default|GetDriving))
    (Default|EndGame (Variables|Default|GetStreetRacerGameMode))
    (Niagara|ResetSystem (Variables|Default|GetExplosion))
    (Rendering|SetVisibility (Variables|Default|GetHeadlight) false false)
    (Rendering|SetVisibility (Variables|Default|GetExplosionLight) true false)
    (Audio|PlaySound2D "/Game/Audio/Crash.Crash" 1.0 1.0 0.0 0 0)
    (bind _explosionbrightness (Timeline|Timeline PlayFromStart)
      (:Update
        (Rendering|Components|Light|SetIntensity (Variables|Default|GetExplosionLight) _explosionbrightness))
      (:Finished
        (Rendering|SetVisibility (Variables|Default|GetExplosionLight) false false)))))

(event Custom|PreventTurning
  (params (Time :type Float%20%28double-precision%29))
  (Utilities|Time|SetTimerbyEvent (delegate Custom|AllowTurning) Time)
  (Variables|Default|SetCanTurnCorner false))

(event Custom|AllowTurning
  (Variables|Default|SetCanTurnCorner true))

(event EventBeginPlay
  (bind _self self)
  (bind _asstreet_racer_controller (Utilities|Casting|CastToStreetRacerController (Game|GetPlayerController 0)))
  (Default|SetCar _asstreet_racer_controller _self)
  (bind _asstreet_racer_game_mode (Utilities|Casting|CastToStreetRacerGameMode (Game|GetGameMode)))
  (bind _output_get (Variables|Default|SetStreetRacerGameMode _asstreet_racer_game_mode))
  (Default|SetPlayerCar _asstreet_racer_game_mode _self))

(event EventTick
  (params (DeltaSeconds :type Float%20%28single-precision%29))
  (if (Variables|Default|GetDriving)
    (Transformation|SetActorLocation (+ (Transformation|GetActorLocation) (* (* DeltaSeconds (Variables|Default|GetSpeed)) (Variables|Default|GetMoveDirection))) false false)
    (CallFunction|TurnPlayerCar DeltaSeconds)))

(fn ConstructionScript)