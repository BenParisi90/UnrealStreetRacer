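; BonusArrow is a bonus arrow pickup that spins in place and disappears when the player touches it.
; Tick yaws the arrow mesh by RotationSpeed, and the box overlap deactivates the actor if it is alive and the other actor is tagged Player.
; ToggleActive reuses the actor instead of destroying it: activation sets a Y position and random yaw, while deactivation drops the root far below.
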(event OnComponentBeginOverlap(Box)
  (params (OverlappedComponent :type Primitive%20Component%20Object%20Reference) (OtherActor :type Actor%20Object%20Reference) (OtherComp :type Primitive%20Component%20Object%20Reference) (OtherBodyIndex :type Integer) (bFromSweep :type Boolean) (SweepResult :type Hit%20Result%20Structure%20%28by%20ref%29))
  (if (and (Actor|ActorHasTag OtherActor "Player") (Variables|Default|GetAlive))
    (CallFunction|ToggleActive false 0.0)))

(event Custom|ToggleActive
  (params (Active :type Boolean) (YLocation :type Float%20%28double-precision%29))
  (bind _output_get (Variables|Default|SetAlive Active))
  (if _output_get
    (Transformation|SetWorldRotation (Variables|Default|GetDefaultSceneRoot) (Math|Rotator|MakeRotator 0.0 0.0 (Math|Random|RandomFloatinRange 0.0 3.6e+02)) false false)
    (Transformation|SetRelativeLocation (Variables|Default|GetDefaultSceneRoot) (Math|Vector|MakeVector 0.0 YLocation 0.0) false false)
    (else
      (Transformation|SetRelativeLocation (Variables|Default|GetDefaultSceneRoot) (Math|Vector|MakeVector 0.0 0.0 -1e+04) false false))))

(event EventTick
  (params (DeltaSeconds :type Float%20%28single-precision%29))
  (Transformation|AddWorldRotation (Variables|Default|GetFX_Arrow_Mesh_01) (Math|Rotator|MakeRotator 0.0 0.0 (* (Variables|Default|GetRotationSpeed) DeltaSeconds)) false false))

(fn ConstructionScript)