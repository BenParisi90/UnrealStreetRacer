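; Player controller for the Street Racer game that turns Enhanced Input actions into game and car commands.
; On BeginPlay it adds the street racer mapping context and caches the StreetRacerGameMode.
; Start/reset and end actions call the game mode, while left and right turn actions call Turn on the car reference supplied through SetCar.
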(event Custom|SetCar
  (params (PlayerCar :type Camera%20Rig%20Object%20Reference))
  (Variables|Default|SetPlayerCar PlayerCar))

(event Input|EnhancedActionEvents|EnhancedInputActionStartOrResetGame
  (params (ActionValue :type Boolean) (ElapsedSeconds :type Float%20%28double-precision%29) (TriggeredSeconds :type Float%20%28double-precision%29) (InputAction :type Input%20Action%20Object%20Reference :default "/Game/Blueprints/Input/StartOrResetGame.StartOrResetGame"))
  (:Triggered
    (Development|PrintString "Start Game")
    (Default|StartorResetGame (Variables|Default|GetStreetRacerGameMode))))

(event Input|EnhancedActionEvents|EnhancedInputActionEndGame
  (params (ActionValue :type Boolean) (ElapsedSeconds :type Float%20%28double-precision%29) (TriggeredSeconds :type Float%20%28double-precision%29) (InputAction :type Input%20Action%20Object%20Reference :default "/Game/Blueprints/Input/EndGame.EndGame"))
  (:Triggered
    (Development|PrintString "End Game")
    (Default|EndGame (Variables|Default|GetStreetRacerGameMode))))

(event Input|EnhancedActionEvents|EnhancedInputActionTurnLeft
  (params (ActionValue :type Boolean) (ElapsedSeconds :type Float%20%28double-precision%29) (TriggeredSeconds :type Float%20%28double-precision%29) (InputAction :type Input%20Action%20Object%20Reference :default "/Game/Blueprints/Input/TurnLeft.TurnLeft"))
  (:Triggered
    (Default|Turn (Variables|Default|GetPlayerCar) true)))

(event Input|EnhancedActionEvents|EnhancedInputActionTurnRight
  (params (ActionValue :type Boolean) (ElapsedSeconds :type Float%20%28double-precision%29) (TriggeredSeconds :type Float%20%28double-precision%29) (InputAction :type Input%20Action%20Object%20Reference :default "/Game/Blueprints/Input/TurnRight.TurnRight"))
  (:Triggered
    (Default|Turn (Variables|Default|GetPlayerCar) false)))

(event EventBeginPlay
  (Input|AddMappingContext (PlayerController|LocalPlayerSubsystems|GetEnhancedInputLocalPlayerSubsystem) "/Game/Blueprints/Input/StreetRacerMappingContext.StreetRacerMappingContext" 0 "(bIgnoreAllPressedKeysUntilRelease=True,bForceImmediately=False)")
  (bind _asstreet_racer_game_mode (Utilities|Casting|CastToStreetRacerGameMode (Game|GetGameMode)))
  (Variables|Default|SetStreetRacerGameMode _asstreet_racer_game_mode))

(event EventTick
  (params (DeltaSeconds :type Float%20%28single-precision%29)))

(fn ConstructionScript)