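; Array helper functions for cycling through indices and randomly showing one mesh from a set.
; IncrementArrayIndex advances an index and wraps to zero at the end of the array.
; TurnOnOne shows one random mesh and hides the rest, without affecting children.
; Despite its name, CanChooseNone never yields an empty pick from multiple meshes: true draws from all, false excludes the last.
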(fn IncrementArrayIndex
  (params (Array :type Array%20of%20Actor%20Object%20References) (Index :type Integer))
  (bind _returnvalue (+ Index 1))
  (if (>= _returnvalue (Utilities|Array|Length Array))
    (return 0)
    (else
      (return _returnvalue))))

(fn TurnonOne
  (params (Meshes :type Array%20of%20Static%20Mesh%20Component%20Object%20References) (CanChooseNone :type Boolean))
  (if CanChooseNone
    (LocalVariables|SetLengthSubtraction 0)
    (else
      (LocalVariables|SetLengthSubtraction 1)))
  (LocalVariables|SetTargetIndex (Math|Random|RandomInteger (- (Utilities|Array|Length Meshes) (LocalVariables|GetLengthSubtraction))))
  (for (_array_element _array_index) Meshes
    (Rendering|SetVisibility _array_element (== (LocalVariables|GetTargetIndex) _array_index) false)))