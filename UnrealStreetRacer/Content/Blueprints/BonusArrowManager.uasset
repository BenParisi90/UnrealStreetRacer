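; BonusArrowManager places bonus arrows along road segments from a recycled pool.
; On BeginPlay it parks every arrow in the BonusArrows array far below the world.
; AddBonusArrows moves a run of arrows to evenly spaced offsets in the given segment's transform, advancing a wrapping index.
; ToggleActive is called after the index increments, so it activates the arrow following the one just placed.
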(event Custom|AddBonusArrows
  (params (RoadSegment :type Road%20Segment%20Object%20Reference))
  (for _index (range 0 5)
    (Transformation|SetActorLocation (Utilities|Array|Get(acopy) (Variables|Default|GetBonusArrows) (Variables|Default|GetBonusArrowIndex)) (Math|Transform|TransformLocation (Transformation|GetActorTransform RoadSegment) (* (Variables|Default|GetArrowOffset) _index)) false false)
    (bind _output_get (Variables|Default|SetBonusArrowIndex (+ (stale _output_get) 1)))
    (Default|ToggleActive (Utilities|Array|Get(acopy) (Variables|Default|GetBonusArrows) (Variables|Default|GetBonusArrowIndex)) true 0.0)
    (if (>= (+ _output_get 1) (Utilities|Array|Length (Variables|Default|GetBonusArrows)))
      (Variables|Default|SetBonusArrowIndex 0))))

(event EventBeginPlay
  (for _array_element (Variables|Default|GetBonusArrows)
    (Transformation|SetActorLocation _array_element "0.000000,0.000000,-10000.000000" false false)))

(fn ConstructionScript)