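; Game mode for a street racer that runs the round state and time-based scoring.
; On BeginPlay it creates the HUD widget for the first player and shows a press-Spacebar prompt.
; While GamePlaying is set, Tick adds PointsPerSecond scaled by delta time to Score and updates the widget.
; StartGame and EndGame toggle that flag and swap the prompt, with StartGame also zeroing the score.
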(event Custom|StartGame
  (Variables|Default|SetGamePlaying true)
  (Default|UpdatePrompt (Variables|Default|GetStreetracerUI))
  (Variables|Default|SetScore 0.0))

(event Custom|EndGame
  (Variables|Default|SetGamePlaying false)
  (Default|UpdatePrompt (Variables|Default|GetStreetracerUI) "Spacebar to Restart"))

(event EventBeginPlay
  (bind _returnvalue (UserInterface|CreateWidget "/Game/Blueprints/StreetRacerUIWidget.StreetRacerUIWidget_C" (Class|GameplayStatics|GetPlayerControllerfromID)))
  (bind _output_get (Variables|Default|SetStreetracerUI _returnvalue))
  (UserInterface|Viewport|AddtoViewport _output_get 0)
  (Default|UpdatePrompt _output_get "Press Spacebar to Begin")
  (Default|UpdateScore _output_get 0.0))

(event EventTick
  (params (DeltaSeconds :type Float%20%28single-precision%29))
  (if (Variables|Default|GetGamePlaying)
    (bind _output_get (Variables|Default|SetScore (+ (Variables|Default|GetScore) (* (Variables|Default|GetPointsPerSecond) DeltaSeconds))))
    (Default|UpdateScore (Variables|Default|GetStreetracerUI) _output_get)))

(fn ConstructionScript)