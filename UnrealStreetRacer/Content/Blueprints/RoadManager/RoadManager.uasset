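; Road manager for a street racer that builds the track from pooled straight, left and right segments and registers itself with the game mode.
; SpawnRoad lays a fixed count of straights, then a random left or right turn, cycling through each pool by index.
; Each segment's end transform positions the next one.
; Segments are moved rather than spawned, and return to a parking position after surviving three spawn cycles.
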(event Custom|PlaceRoadSegment
  (params (RoadSegment :type Array%20of%20Road%20Segment%20Object%20References) (Index :type Integer) (FirstSegment :type Boolean))
  (bind _output (Utilities|Array|Get(acopy) RoadSegment Index))
  (bind _returnvalue (Transformation|GetActorTransform _output))
  (Development|PrintString (Utilities|GetObjectName _output) true true "(R=0.000000,G=0.660000,B=1.000000,A=1.000000)" 1e+03)
  (Transformation|SetActorLocation _output (Variables|Default|GetNextPlacementPosition) false false)
  (Transformation|SetActorRotation _output (Variables|Default|GetNextPlacementRotation))
  (Variables|Default|SetNextPlacementPosition (Math|Transform|TransformLocation _returnvalue (Variables|/Game/Blueprints/RoadManager/RoadSegment.RoadSegment_C|GetEndPos _output)))
  (Variables|Default|SetNextPlacementRotation (Math|Transform|TransformRotation _returnvalue (Variables|/Game/Blueprints/RoadManager/RoadSegment.RoadSegment_C|GetEndRot _output)))
  (Variables|/Game/Blueprints/RoadManager/RoadSegment.RoadSegment_C|SetAlive _output true))

(event Custom|SpawnRoad
  (bind _roadstraight (Variables|Default|GetRoadStraight))
  (bind _roadleft (Variables|Default|GetRoadLeft))
  (bind _roadright (Variables|Default|GetRoadRight))
  (CallFunction|ClearOldRoad (Variables|Default|GetRoadStraight))
  (CallFunction|ClearOldRoad (Variables|Default|GetRoadLeft))
  (CallFunction|ClearOldRoad (Variables|Default|GetRoadRight))
  (for _index (range 0 (- (Variables|Default|GetMaxStraightSegments) 1))
    (CallFunction|PlaceRoadSegment _roadstraight (Variables|Default|GetRoadStraightIndex) false)
    (bind _output (CallFunction|IncrementArrayIndex _roadstraight (Variables|Default|GetRoadStraightIndex)))
    (Variables|Default|SetRoadStraightIndex _output))
  (if (Math|Random|RandomBool)
    (CallFunction|PlaceRoadSegment _roadleft (Variables|Default|GetRoadLeftIndex) false)
    (bind _output_2 (CallFunction|IncrementArrayIndex _roadleft (Variables|Default|GetRoadLeftIndex)))
    (Variables|Default|SetRoadLeftIndex _output_2)
    (else
      (CallFunction|PlaceRoadSegment _roadright (Variables|Default|GetRoadRightIndex) false)
      (bind _output_3 (CallFunction|IncrementArrayIndex _roadright (Variables|Default|GetRoadRightIndex)))
      (Variables|Default|SetRoadRightIndex _output_3))))

(event Custom|ClearOldRoad
  (params (RoadSegments :type Array%20of%20Road%20Segment%20Object%20References))
  (for _array_element RoadSegments
    (if (Variables|/Game/Blueprints/RoadManager/RoadSegment.RoadSegment_C|GetAlive _array_element)
      (bind _output_get (Variables|/Game/Blueprints/RoadManager/RoadSegment.RoadSegment_C|SetTurnsAlive _array_element (+ (Variables|/Game/Blueprints/RoadManager/RoadSegment.RoadSegment_C|GetTurnsAlive _array_element) 1)))
      (if (>= _output_get 3)
        (Variables|/Game/Blueprints/RoadManager/RoadSegment.RoadSegment_C|SetAlive _array_element false)
        (Variables|/Game/Blueprints/RoadManager/RoadSegment.RoadSegment_C|SetTurnsAlive _array_element 0)
        (Transformation|SetActorLocation _array_element (Variables|Default|GetResetRoadPosition) false false)))))

(event Custom|Reset
  (bind _resetroadposition (Variables|Default|GetResetRoadPosition))
  (Variables|Default|SetNextPlacementPosition "0, 0, 0")
  (for _array_element (Variables|Default|GetRoadStraight)
    (Transformation|SetActorLocation _array_element _resetroadposition false false))
  (Transformation|SetActorLocation _resetroadposition false false)
  (Transformation|SetActorLocation _resetroadposition false false)
  (Variables|Default|SetNextPlacementPosition "0, 0, 0")
  (Variables|Default|SetNextPlacementRotation "0, 0, 0"))

(event EventBeginPlay
  (bind _asstreet_racer_game_mode (Utilities|Casting|CastToStreetRacerGameMode (Game|GetGameMode)))
  (Default|SetRoadManager _asstreet_racer_game_mode self))

(fn ConstructionScript)